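; Weather system actor that spawns lightning strikes at random intervals.
; BeginPlay loops on a random retriggerable delay, each pass setting a separately randomized timer for LightningTimer.
; LightningTimer traces from the actor toward a random forward-cone vector scaled by TraceLength, used as a world position without adding actor location.
; On a hit it spawns an attached Niagara lightning effect, passing start and end points, with ImpactNormal receiving the impact point.
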(event EventBeginPlay
  (bind _mintimerspawn (Variables|Default|GetMinTimerSpawn))
  (bind _maxtimerspawn (Variables|Default|GetMaxTimerSpawn))
  (bind _returnvalue (Math|Random|RandomFloatinRange _mintimerspawn _maxtimerspawn))
  (Utilities|Time|SetTimerbyFunctionName 0 "LightningTimer" _returnvalue :!label _label)
  (Utilities|FlowControl|RetriggerableDelay _returnvalue)
  (goto _label))

(event Collision|EventActorBeginOverlap
  (params (OtherActor :type Actor%20Object%20Reference)))

(event EventTick
  (params (DeltaSeconds :type Float%20%28single-precision%29)))

(fn ConstructionScript)

(fn LightningTimer
  (bind (_outhit _returnvalue) (Collision|LineTraceByChannel (Transformation|GetActorLocation) (* (Math|Random|RandomUnitVectorinConeinDegrees (Transformation|GetActorForwardVector) (Variables|Default|GetTraceConeAngle)) (Variables|Default|GetTraceLength)) "TraceTypeQuery1" false 0 "None"))
  (if _returnvalue
    (bind _returnvalue_2 (Niagara|SpawnSystemAttached (Variables|Default|GetLightningEmitter) (Variables|Transformation|GetRootComponent) "None" "0, 0, 0" "0, 0, 0" "KeepRelativeOffset" true))
    (Niagara|SetNiagaraVariable(Vector3) _returnvalue_2 "LightningStartPoint" "0, 0, 0")
    (Niagara|SetNiagaraVariable(Vector3) _returnvalue_2 "LightningEndPoint" (.Location (Collision|BreakHitResult _outhit)))
    (Niagara|SetNiagaraVariable(Vector3) _returnvalue_2 "ImpactNormal" (.ImpactPoint (Collision|BreakHitResult _outhit)))))