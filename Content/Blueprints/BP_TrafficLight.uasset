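; Traffic light actor that displays separate vehicle and pedestrian signal states on one light mesh.
; On BeginPlay it creates a dynamic material instance for each of the mesh's two signal material slots.
; State setters drive material parameters for colour, blinking and a colour-channel mask selecting the lamp; getters expose the current states.
; Error blinks the middle traffic lamp and zeroes pedestrian emissive; the Blueprint has no cycling logic of its own.
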(event EventBeginPlay
  (bind _returnvalue (Rendering|Material|CreateDynamicMaterialInstance (Variables|Default|GetLightMesh) 0 "/Game/Materials/MI_Pedestrian_01a.MI_Pedestrian_01a" "None" :!class /Script/Engine.PrimitiveComponent))
  (Variables|Default|SetPedestrianMaterial _returnvalue)
  (bind _returnvalue_2 (Rendering|Material|CreateDynamicMaterialInstance (Variables|Default|GetLightMesh) 1 "/Game/Materials/MI_TrafficLight_01a.MI_TrafficLight_01a" "None" :!class /Script/Engine.PrimitiveComponent))
  (Variables|Default|SetTrafficMaterial _returnvalue_2))

(event Collision|EventActorBeginOverlap
  (params (OtherActor :type Actor%20Object%20Reference)))

(event EventTick
  (params (DeltaSeconds :type Float%20%28single-precision%29)))

(fn ConstructionScript)

(fn GetTrafficState
  (return (Variables|Default|GetCurrentTrafficState)))

(fn GetPedestrianState
  (return (Variables|Default|GetCurrentPedestrianState)))

(fn SetTrafficState
  (params (New%20State :type E_TrafficStates%20Enum :default "NewEnumerator0"))
  (bind _trafficmaterial (Variables|Default|GetTrafficMaterial))
  (bind _output_get (Variables|Default|SetCurrentTrafficState New%20State))
  (Rendering|Material|SetVectorParameterValue (Variables|Default|GetTrafficMaterial) "LightColour" (Utilities|Array|Get(acopy) (Variables|Default|GetLightColours) (Math|Conversions|ToInteger(Byte) _output_get)) :!class /Script/Engine.MaterialInstanceDynamic)
  (switch Utilities|FlowControl|Switch|SwitchonE_TrafficStates _output_get
    (:NewEnumerator0
      (Rendering|Material|SetVectorParameterValue _trafficmaterial "LightSwitch" "(R=1.000000,G=0.000000,B=0.000000,A=1.000000)" :!class /Script/Engine.MaterialInstanceDynamic)
      (Rendering|Material|SetScalarParameterValue (Variables|Default|GetTrafficMaterial) "IsBlinking" 0.0 :!class /Script/Engine.MaterialInstanceDynamic :!label _label))
    (:NewEnumerator1
      (Rendering|Material|SetVectorParameterValue _trafficmaterial "LightSwitch" "(R=0.000000,G=1.000000,B=0.000000,A=1.000000)" :!class /Script/Engine.MaterialInstanceDynamic)
      (goto _label))
    (:NewEnumerator2
      (Rendering|Material|SetVectorParameterValue _trafficmaterial "LightSwitch" "(R=0.000000,G=0.000000,B=1.000000,A=1.000000)" :!class /Script/Engine.MaterialInstanceDynamic)
      (goto _label))
    (:NewEnumerator3
      (Rendering|Material|SetVectorParameterValue _trafficmaterial "LightSwitch" "(R=0.000000,G=1.000000,B=0.000000,A=1.000000)" :!class /Script/Engine.MaterialInstanceDynamic)
      (Rendering|Material|SetScalarParameterValue (Variables|Default|GetTrafficMaterial) "IsBlinking" 1.0 :!class /Script/Engine.MaterialInstanceDynamic))))

(fn SetPedestrianState
  (params (New%20State :type E_PedestrianStates%20Enum :default "NewEnumerator0"))
  (bind _pedestrianmaterial (Variables|Default|GetPedestrianMaterial))
  (bind _pedestrianmaterial_2 (Variables|Default|GetPedestrianMaterial))
  (bind _pedestrianmaterial_3 (Variables|Default|GetPedestrianMaterial))
  (bind _output_get (Variables|Default|SetCurrentPedestrianState New%20State))
  (Rendering|Material|SetVectorParameterValue (Variables|Default|GetPedestrianMaterial) "LightColour" (Utilities|Array|Get(acopy) (Variables|Default|GetLightColours) (Math|Conversions|ToInteger(Byte) _output_get)) :!class /Script/Engine.MaterialInstanceDynamic)
  (switch Utilities|FlowControl|Switch|SwitchonE_PedestrianStates _output_get
    (:NewEnumerator0
      (Rendering|Material|SetVectorParameterValue _pedestrianmaterial_2 "LightSwitch" "(R=1.000000,G=0.000000,B=0.000000,A=1.000000)" :!class /Script/Engine.MaterialInstanceDynamic)
      (Rendering|Material|SetScalarParameterValue _pedestrianmaterial_3 "IsBlinking" 0.0 :!class /Script/Engine.MaterialInstanceDynamic :!label _label)
      (Rendering|Material|SetScalarParameterValue _pedestrianmaterial_3 "EmissiveMulti" 5.0 :!class /Script/Engine.MaterialInstanceDynamic :!label _label_2))
    (:NewEnumerator1
      (Rendering|Material|SetVectorParameterValue _pedestrianmaterial_2 "LightSwitch" "(R=0.000000,G=1.000000,B=0.000000,A=1.000000)" :!class /Script/Engine.MaterialInstanceDynamic)
      (Rendering|Material|SetScalarParameterValue _pedestrianmaterial "IsBlinking" 1.0 :!class /Script/Engine.MaterialInstanceDynamic)
      (Rendering|Material|SetVectorParameterValue _pedestrianmaterial "LightColour" (Utilities|Array|Get(acopy) (Variables|Default|GetLightColours)) :!class /Script/Engine.MaterialInstanceDynamic)
      (goto _label_2))
    (:NewEnumerator2
      (Rendering|Material|SetVectorParameterValue _pedestrianmaterial_2 "LightSwitch" "(R=0.000000,G=0.000000,B=1.000000,A=1.000000)" :!class /Script/Engine.MaterialInstanceDynamic)
      (goto _label))
    (:NewEnumerator3
      (Rendering|Material|SetScalarParameterValue _pedestrianmaterial_2 "EmissiveMulti" 0.0 :!class /Script/Engine.MaterialInstanceDynamic))))